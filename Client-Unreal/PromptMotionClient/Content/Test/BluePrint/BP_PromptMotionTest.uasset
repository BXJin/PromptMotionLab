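; BP_PromptMotionTest is a test actor that exercises a PromptMotionRuntime component's messaging and face presets.
; On BeginPlay it sends a Korean greeting as a runtime message and enables player input.
; Each runtime response has its behavior emotion, gaze and gesture key printed on screen.
; Number keys 1 to 4 bypass messaging and directly apply friendly, thinking, concerned or neutral face presets.
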(event `self.ReceiveBeginPlay`
  (`PromptMotionRuntimeComponent.SendRuntimeMessage` (`self.PromptMotionRuntime`) "안녕하세요")
  (`self.EnableInput` (`GameplayStatics.GetPlayerController` 0)))

(event `self.PromptMotionRuntime.OnRuntimeResponseReceived`
  (params (Response :type "PromptMotionRuntimeResponse Structure (by ref)"))
  (bind (_bsuccess _reply _behavior) (break `PromptMotionRuntimeResponse` Response))
  (`KismetSystemLibrary.PrintString` (`KismetStringLibrary.Concat_StrStr` "emotion:" (break `PromptMotionBehavior` _behavior) "/" (`.Gaze` (break `PromptMotionBehavior` _behavior)) "/" "gesture: " (`.GestureKey` (break `PromptMotionBehavior` _behavior)))))

(event `Key|One`
  (params (Key :type "Key Structure"))
  (:`Pressed`
    (`PromptMotionRuntimeComponent.ApplyFacePreset` (`self.PromptMotionRuntime`) "friendly" 0.7)))

(event `Key|Two`
  (params (Key :type "Key Structure"))
  (:`Pressed`
    (`PromptMotionRuntimeComponent.ApplyFacePreset` (`self.PromptMotionRuntime`) "thinking" 0.7)))

(event `Key|Three`
  (params (Key :type "Key Structure"))
  (:`Pressed`
    (`PromptMotionRuntimeComponent.ApplyFacePreset` (`self.PromptMotionRuntime`) "concerned" 0.7)))

(event `Key|Four`
  (params (Key :type "Key Structure"))
  (:`Pressed`
    (`PromptMotionRuntimeComponent.ApplyFacePreset` (`self.PromptMotionRuntime`) "neutral" 0.0)))

(fn `UserConstructionScript`)